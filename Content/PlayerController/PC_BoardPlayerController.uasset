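; Player controller for a turn-based board game that turns mouse clicks into ship selection, movement and spawning.
; Left click traces under the cursor: ships toggle selection, while cells go to ClickOnCell.
; With a ship selected, a cell click asks the board manager to move it for the current player; otherwise the visualiser spawns a ship on unoccupied cells.
; Two other inputs switch between preset spring-arm and camera angles on the player pawn.
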(event `self.ReceiveBeginPlay`
  (`EnhancedInputSubsystemInterface.AddMappingContext` (subsystem `EnhancedInputLocalPlayerSubsystem`) "/Game/Input/IMC_BoardGame.IMC_BoardGame" 0 (struct))
  (set `self.BoardGamemodeRef` (cast `/Game/Gamemode/GM_BoardGameMode` (`GameplayStatics.GetGameMode`) :!pure true))
  (set `self.PlayerRef` (cast `/Game/Dev/Blueprints/Player/BP_PlayerTest` (`GameplayStatics.GetPlayerCharacter` 0) :!pure true)))

(event `EnhancedInput|/Game/Input/IA_LeftClick`
  (params (ActionValue :type Boolean) (ElapsedSeconds :type "Float (double-precision)") (TriggeredSeconds :type "Float (double-precision)") (InputAction :type "InputAction Object Reference" :default "/Game/Input/IA_LeftClick.IA_LeftClick"))
  (bind _hitresult (`self.GetHitResultUnderCursorByChannel` "TraceTypeQuery1"))
  (:`Started`
    (bind _asbp_ship (cast `/Game/Dev/Blueprints/BoardActor/BP_Ship` (`.HitActor` (`GameplayStatics.BreakHitResult` _hitresult)))
      (:`then`
        (`self.ClickOnShip` _asbp_ship))
      (:`CastFailed`
        (bind _asbp_board_cell (cast `/Game/Cells/BP_BoardCell` (`.HitActor` (`GameplayStatics.BreakHitResult` _hitresult)))
          (:`then`
            (`self.ClickOnCell` _asbp_board_cell))
          (:`CastFailed`
            (`KismetSystemLibrary.PrintString` "Nothing")))))))

(event `EnhancedInput|/Game/Input/IA_A`
  (params (ActionValue :type Boolean) (ElapsedSeconds :type "Float (double-precision)") (TriggeredSeconds :type "Float (double-precision)") (InputAction :type "InputAction Object Reference" :default "/Game/Input/IA_A.IA_A"))
  (:`Started`
    (`self.ChangeCameraAngle` 0)))

(event `EnhancedInput|/Game/Input/IA_E`
  (params (ActionValue :type Boolean) (ElapsedSeconds :type "Float (double-precision)") (TriggeredSeconds :type "Float (double-precision)") (InputAction :type "InputAction Object Reference" :default "/Game/Input/IA_E.IA_E"))
  (:`Started`
    (`self.ChangeCameraAngle` 1)))

(fn `ChangeCameraAngle`
  (params (CameraAngleIndex :type Integer))
  (bind _playerref (`self.PlayerRef`))
  (set `SpringArmComponent.SocketOffset` (`|GetArrayItem` (`self.CameraAngleLocation`) CameraAngleIndex) (`/Game/Dev/Blueprints/Player/BP_PlayerTest.SpringArm` _playerref))
  (`SceneComponent.K2_SetRelativeRotation` (`/Game/Dev/Blueprints/Player/BP_PlayerTest.Camera` _playerref) (`|GetArrayItem` (`self.CameraAngleRotation`) CameraAngleIndex) false false))

(fn `ClickOnCell`
  (params (SelectedCell :type "ABoardCell Object Reference"))
  (bind _celldata_pos (break `Cell` (`ABoardCell.cellData` SelectedCell)))
  (bind _boardgamemoderef (`self.BoardGamemodeRef`))
  (bind _selectedship (`self.SelectedShip`))
  (bind _returnvalue (`ABoardGameMode.BoardManagerGet` _boardgamemoderef))
  (bind _asgm_board_game_mode (cast `/Game/Gamemode/GM_BoardGameMode` (`GameplayStatics.GetGameMode`) :!pure true))
  (bind _boardvisualiser (`/Game/Gamemode/GM_BoardGameMode.BoardVisualiser` _boardgamemoderef))
  (bind _returnvalue_pos (break `Cell` (`UBoardManager.GetCell` _returnvalue _celldata_pos)))
  (`/Engine/EditorBlueprintResources/StandardMacros.IsValid` _selectedship
    (:`Is Valid`
      (`KismetSystemLibrary.PrintString` "CellAndHaveShip")
      (`KismetSystemLibrary.PrintString` (`KismetStringLibrary.Conv_IntPointToString` _celldata_pos))
      (`UBoardManager.MoveShipTo` (`ABoardGameMode.BoardManagerGet` _asgm_board_game_mode) _selectedship _celldata_pos (`UTurnManager.GetCurrentPlayer` (`ABoardGameMode.GetTurnManager` _asgm_board_game_mode))))
    (:`Is Not Valid`
      (if (`UBoardManager.IsCellOccupied` _returnvalue _celldata_pos)
        (`KismetSystemLibrary.PrintString` "CellOccuped")
        (else
          (`ABoardVisualiser.SpawnShip` _boardvisualiser (`ABoardVisualiser.ShipClass` _boardvisualiser) _returnvalue_pos (`self.Card Data`))
          (`KismetSystemLibrary.PrintString` "CellNotOccupedSoTrySpawnShip"))))))

(fn `ClickOnShip`
  (params (SelectedShip :type "AShip Object Reference"))
  (if (== (`self.SelectedShip`) SelectedShip)
    (if (`AShip.bJustPlayed` (`self.SelectedShip`))
      _
      (else
        _))
    (set `self.SelectedShip` null)
    (`KismetSystemLibrary.PrintString` "UnSetSelectedShip")
    (else
      (set `self.SelectedShip` SelectedShip)
      (`KismetSystemLibrary.PrintString` "SetSelectedShip"))))

(fn `UserConstructionScript`)