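; BP_Refinery is a refinery board actor that shows which player controls it through its material.
; UpdateControlIndicator maps the player ID to a blue, red or neutral material.
; Material has an OnRep function that applies it to the second material slot of the Sphere mesh, so the indicator follows replication.
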(event `self.UpdateControlIndicator`
  (params (PlayerID :type Integer))
  (if (== PlayerID 0)
    (set `self.Material` "/Game/BoardActors/Refinery/Materials/M_RefineryBlue.M_RefineryBlue")
    (elif (== PlayerID 1)
      (set `self.Material` "/Game/BoardActors/Refinery/Materials/M_RefineryRed.M_RefineryRed")
      (else
        (set `self.Material` "/Game/BoardActors/Refinery/Materials/M_RefineryNormal.M_RefineryNormal")))))

(fn `OnRep_Material`
  (`PrimitiveComponent.SetMaterial` (`self.Sphere`) 1 (`self.Material`)))

(fn `UserConstructionScript`)