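; GM_BoardGameMode is the game mode for a board game that relays card draws to player controllers.
; When initialisation finishes, it binds to the DeckManager's OnCardDrawn event, presumably to its OnCardDraw handler.
; OnCardDraw looks up the player controller by player id, casts it to PC_BoardPlayerController and passes it the card data.
; Both steps print debug strings, and PostLogin only calls the parent.
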(event `self.K2_PostLogin`
  (params (NewPlayer :type "PlayerController Object Reference"))
  (`parent.K2_PostLogin` NewPlayer))

(event `self.OnInitialisationFinishedBP`
  (add `DeckManager.OnCardDrawn` (`self.deckManager`) (`|CreateDelegate` :!event `OnCardDraw`))
  (`KismetSystemLibrary.PrintString` "binded" true true (struct :`R` 0.249166 :`G` 0.042014 :`B` 1.0 :`A` 1.0) 20000.0))

(fn `OnCardDraw`
  (params (PlayerId :type Integer) (CardData :type "UCardData Object Reference"))
  (`KismetSystemLibrary.PrintString` "gm : draw card")
  (bind _aspc_board_player_controller (cast `/Game/Player/PlayerController/PC_BoardPlayerController` (`GameplayStatics.GetPlayerController` PlayerId)))
  (`/Game/Player/PlayerController/PC_BoardPlayerController.DrawCard` _aspc_board_player_controller CardData))

(fn `UserConstructionScript`)