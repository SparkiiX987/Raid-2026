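; Lobby game mode for a two-player online session, handling joins, leaves, host assignment and kicks.
; Shortly after PostLogin it increments a connection count, kicks overflow or uninvited private-server players, and flags the first player as host.
; Joins and logouts update the session's isFull property and advertise it only when public.
; Helpers let the second player be kicked with a lobby UI refresh and decrement the GameState's ready count.
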(event `self.ReceiveBeginPlay`
  (`KismetSystemLibrary.K2_SetTimerDelegate` (delegate `NumberOfPlayer`) 1.0 true)
  (bind _asgi_main_menu_game_instance (cast `/Game/GameInstance/GI_MainMenuGameInstance` (`GameplayStatics.GetGameInstance`)))
  (set `self.GameInstanceRef` _asgi_main_menu_game_instance)
  (set `self.GameStateRef` (cast `/Game/GS_LobbyGameState` (`GameplayStatics.GetGameState`) :!pure true)))

(event `NumberOfPlayer`
  (`KismetSystemLibrary.PrintString` (`KismetStringLibrary.Concat_StrStr` "The number of plaeyer is " (`KismetStringLibrary.Conv_IntToString` (`KismetArrayLibrary.Array_Length` (`GameStateBase.PlayerArray` (`GameplayStatics.GetGameState`)))))))

(event `self.K2_PostLogin`
  (params (NewPlayer :type "PlayerController Object Reference"))
  (`KismetSystemLibrary.K2_SetTimerDelegate` (delegate `CheckCondition`) 0.5))

(event `CheckCondition`
  (bind _result (`/Engine/EditorBlueprintResources/StandardMacros.IncrementInt` (`self.PlayerConnect`))
    (:`  `
      (if (> _result 2)
        (`AdvancedSessionsLibrary.KickPlayer` (stale `self.K2_PostLogin` NewPlayer) "Full")
        (`KismetSystemLibrary.PrintString` "C'EST FULL" true true (struct :`R` 0.223193 :`G` 1.0 :`A` 1.0) 10.0)
        (elif (and (== (`/Game/PS_LobbyPlayerState.bIsInvited` (cast `/Game/PS_LobbyPlayerState` (`Controller.PlayerState` (stale `self.K2_PostLogin` NewPlayer)) :!pure true)) false) (== (`/Game/GameInstance/GI_MainMenuGameInstance.bIsPrivateServer` (cast `/Game/GameInstance/GI_MainMenuGameInstance` (`GameplayStatics.GetGameInstance`) :!pure true)) true))
          (`AdvancedSessionsLibrary.KickPlayer` (stale `self.K2_PostLogin` NewPlayer) "Full")
          (`KismetSystemLibrary.PrintString` "T'ES PAS INVITE" true true (struct :`R` 0.223193 :`G` 1.0 :`A` 1.0) 10.0)
          (elif (> (`self.PlayerConnect`) 1)
            (bind (_numconnections _numprivateconnections _bislan _bisdedicated _ballowinvites _ballowjoininprogress) (`AdvancedSessionsLibrary.GetSessionSettings`)
              (:`OnSuccess`
                (`UpdateSessionCallbackProxyAdvanced.UpdateSession` (`|MakeArray` (`AdvancedSessionsLibrary.MakeLiteralSessionPropertyBool` "isFull" true)) _numconnections _numprivateconnections _bislan _ballowinvites _ballowjoininprogress true _bisdedicated (== (`/Game/GameInstance/GI_MainMenuGameInstance.bIsPrivateServer` (cast `/Game/GameInstance/GI_MainMenuGameInstance` (`GameplayStatics.GetGameInstance`) :!pure true)) false)
                  (:`OnSuccess`
                    (`KismetSystemLibrary.PrintString` "Succes Update session data for full" true true (struct :`G` 0.66 :`B` 1.0 :`A` 1.0) 10.0))
                  (:`OnFailure`
                    (`KismetSystemLibrary.PrintString` "Failed update session data for full" true true (struct :`G` 0.66 :`B` 1.0 :`A` 1.0) 10.0))))
              (:`OnFailure`
                (`KismetSystemLibrary.PrintString` "Fail get session settings")))
            (else
              (set `/Game/PS_LobbyPlayerState.bIsHost` true (cast `/Game/PS_LobbyPlayerState` (`Controller.PlayerState` (stale `self.K2_PostLogin` NewPlayer)) :!pure true))
              (bind (_numconnections_2 _numprivateconnections_2 _bislan_2 _bisdedicated_2 _ballowinvites_2 _ballowjoininprogress_2) (`AdvancedSessionsLibrary.GetSessionSettings`)
                (:`OnSuccess`
                  (`UpdateSessionCallbackProxyAdvanced.UpdateSession` (`|MakeArray` (`AdvancedSessionsLibrary.MakeLiteralSessionPropertyBool` "isFull")) _numconnections_2 _numprivateconnections_2 _bislan_2 _ballowinvites_2 _ballowjoininprogress_2 true _bisdedicated_2 (== (`/Game/GameInstance/GI_MainMenuGameInstance.bIsPrivateServer` (cast `/Game/GameInstance/GI_MainMenuGameInstance` (`GameplayStatics.GetGameInstance`) :!pure true)) false)
                    (:`OnSuccess`
                      (`KismetSystemLibrary.PrintString` "Succes Update session data for one player" true true (struct :`G` 0.66 :`B` 1.0 :`A` 1.0) 10.0))
                    (:`OnFailure`
                      (`KismetSystemLibrary.PrintString` "Failed update session data for one player" true true (struct :`G` 0.66 :`B` 1.0 :`A` 1.0) 10.0))))
                (:`OnFailure`
                  (`KismetSystemLibrary.PrintString` "Fail get session settings for one player" true true (struct :`G` 0.66 :`B` 1.0 :`A` 1.0) 10.0))))))))))

(event `self.K2_OnLogout`
  (params (ExitingController :type "Controller Object Reference"))
  (bind _bisprivateserver (`/Game/GameInstance/GI_MainMenuGameInstance.bIsPrivateServer` (cast `/Game/GameInstance/GI_MainMenuGameInstance` (`GameplayStatics.GetGameInstance`) :!pure true)))
  (`/Engine/EditorBlueprintResources/StandardMacros.DecrementInt` (`self.PlayerConnect`)
    (:`  `
      (if (< (`self.PlayerConnect`) 2)
        (bind (_numconnections _numprivateconnections _bislan _bisdedicated _ballowinvites _ballowjoininprogress) (`AdvancedSessionsLibrary.GetSessionSettings`)
          (:`OnSuccess`
            (`UpdateSessionCallbackProxyAdvanced.UpdateSession` (`|MakeArray` (`AdvancedSessionsLibrary.MakeLiteralSessionPropertyBool` "isFull") (`AdvancedSessionsLibrary.MakeLiteralSessionPropertyBool` "isPrivate" _bisprivateserver)) _numconnections _numprivateconnections _bislan _ballowinvites _ballowjoininprogress true _bisdedicated (== _bisprivateserver false)
              (:`OnSuccess`
                (`KismetSystemLibrary.PrintString` "Sucess update session for isFull is false" true true (struct :`R` 1.0 :`B` 0.040431 :`A` 1.0) 10.0))
              (:`OnFailure`
                (`KismetSystemLibrary.PrintString` "Fail update session for isFull is false" true true (struct :`R` 1.0 :`B` 0.040431 :`A` 1.0) 10.0))))
          (:`OnFailure`
            (`KismetSystemLibrary.PrintString` "Fail get session settings")))
        (else
          (`KismetSystemLibrary.PrintString` "Not under one Player" true true (struct :`G` 0.068065 :`B` 1.0 :`A` 1.0) 10.0))))))

(event `RemovePlayerReady`
  (`/Engine/EditorBlueprintResources/StandardMacros.DecrementInt` (`/Game/GS_LobbyGameState.numbreOfReadyPlayer` (`self.GameStateRef`))))

(fn `KickPlayer`
  (if (> (`self.PlayerConnect`) 1)
    (`AdvancedSessionsLibrary.KickPlayer` (`PlayerState.GetPlayerController` (`|GetArrayItem` (`GameStateBase.PlayerArray` (`self.GameStateRef`)) 1)) "Je te veux pas")
    (`/Game/GS_LobbyGameState.UpdateEachLobbyUi` (`self.GameStateRef`))))

(fn `UserConstructionScript`)