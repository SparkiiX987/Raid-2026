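; Player Blueprint for a card game, holding a deck Set and a hand of three card meshes.
; BeginPlay fills the hand; ShuffleDeck copies the deck to an array, overwrites random slots, then rebuilds the Set.
; PickCard shows a card on the first hand slot by swapping its material, but requests the index one past the deck's end.
; Drawn cards stay in the deck, as the Remove node is unwired.
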(event `ShuffleDeck`
  (bind _carddeck (`self.CardDeck`))
  (bind _returnvalue (- (`BlueprintSetLibrary.Set_Length` _carddeck) 1))
  (bind _returnvalue_2 (`KismetMathLibrary.RandomIntegerInRange` 0 _returnvalue))
  ; shuffle Deck
  (bind _result (`BlueprintSetLibrary.Set_ToArray` _carddeck))
  (for _index (range (+ _returnvalue 1))
    (bind _output_get (set `self.tmpShuffleCardDeck` (`BlueprintSetLibrary.Set_GetItemByIndex` _carddeck _returnvalue_2)))
    (`KismetArrayLibrary.Array_Set` _result _returnvalue_2 (`BlueprintSetLibrary.Set_GetItemByIndex` _carddeck _index))
    (`KismetArrayLibrary.Array_Set` _result _index _output_get))
  (`BlueprintSetLibrary.Set_Clear` _carddeck)
  (`BlueprintSetLibrary.Set_AddItems` (`self.CardDeck`) _result))

(event `self.ReceiveBeginPlay`
  ; Comment
  (set `self.HandCard` (`|MakeArray` (`self.Card_body`) (`self.Card_body1`) (`self.Card_body2`))))

(event `PickCard`
  ; Picks a Card
  (bind _cardiddeck (`self.GetCard` (`BlueprintSetLibrary.Set_Length` (`self.CardDeck`))))
  (`self.DrawCard` _cardiddeck))

(fn `DrawCard`
  (params (Cards :type "/Game/Dev/DataAsset/DA_Cards Object Reference") (Index :type Integer))
  (`PrimitiveComponent.SetMaterial` (`|GetArrayItem` (`self.HandCard`) Index) 0 (`/Game/Dev/DataAsset/DA_Cards.CardMat` Cards)))

(fn `GetCard`
  (params (CardId :type Integer))
  (returns (CardIdDeck :type "/Game/Dev/DataAsset/DA_Cards Object Reference"))
  (return (`BlueprintSetLibrary.Set_GetItemByIndex` (`self.CardDeck`) CardId)))

(fn `UserConstructionScript`)