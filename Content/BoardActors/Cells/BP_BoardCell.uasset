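; BP_BoardCell is a board cell actor that can visually toggle a highlight on its Cube component.
; The construction script applies the base material to the cube.
; The HighlightCell and ClearCellHighlight events swap the first material slot between the highlighted and base materials.
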(event `self.HighlightCell`
  (`PrimitiveComponent.SetMaterial` (`self.Cube`) 0 (`self.HighlitedMaterial`)))

(event `self.ClearCellHighlight`
  (`PrimitiveComponent.SetMaterial` (`self.Cube`) 0 (`self.BaseMaterial`)))

(fn `UserConstructionScript`
  (`PrimitiveComponent.SetMaterial` (`self.Cube`) 0 (`self.BaseMaterial`)))