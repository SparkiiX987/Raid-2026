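; PC_LobbyPlayerController is the player controller for the lobby, linking each player's lobby UI to game and player state.
; On BeginPlay it enables mouse and UI-only input, and for the local controller creates WBP_Lobby and registers it on GS_LobbyGameState.
; It passes the game instance's IsInvited flag to PS_LobbyPlayerState through a server event.
; Another server event flags the game state as starting the game.
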(event `self.ReceiveBeginPlay`
  (bind _asgs_lobby_game_state (cast `/Game/GS_LobbyGameState` (`GameplayStatics.GetGameState`) :!pure true))
  (set `self.bShowMouseCursor` true)
  (`WidgetBlueprintLibrary.SetInputMode_UIOnlyEx` self null)
  (if (`self.IsLocalController`)
    (bind _returnvalue (`|CreateWidget` "/Game/UI/WBP_Lobby.WBP_Lobby_C"))
    (`UserWidget.AddToViewport` _returnvalue 0)
    (set `/Game/GS_LobbyGameState.LobbyUi` _returnvalue _asgs_lobby_game_state)
    (set `self.GameStateRef` _asgs_lobby_game_state)
    (bind _asgi_main_menu_game_instance (cast `/Game/GameInstance/GI_MainMenuGameInstance` (`GameplayStatics.GetGameInstance`)))
    (`self.Server_SetInvited` (`/Game/GameInstance/GI_MainMenuGameInstance.bIsInvited` _asgi_main_menu_game_instance))))

(event `Server_StartGame`
  (set `/Game/GS_LobbyGameState.bIsStartingGame` true (`self.GameStateRef`)))

(event `Server_SetInvited`
  (params (Invited :type Boolean))
  (set `/Game/PS_LobbyPlayerState.bIsInvited` Invited (cast `/Game/PS_LobbyPlayerState` (`self.PlayerState`) :!pure true)))

(fn `UserConstructionScript`)