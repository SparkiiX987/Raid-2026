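; Game mode for the board game that sets up a match on BeginPlay.
; It spawns managers, then a board visualiser linked to the board and turn managers, whose refineries and two motherships feed board initialization.
; Deck setup repeatedly loads a temporary card list for player 0, then the turn manager starts the game with player 0 first.
; Finally, the test player character is moved onto a fixed grid cell.
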(event `self.ReceiveBeginPlay`
  (`self.SpawnManagers`)
  (`self.InitializeBoard`)
  (`self.InitializeDecks`)
  (`self.InitializeTurnManager`)
  (`self.InitializePlayerPosition`))

(fn `InitializeBoard`
  (bind _returnvalue (`self.BoardManagerGet`))
  (bind _returnvalue_2 (`self.BoardManagerGet`))
  (bind _returnvalue_3 (`self.GetTurnManager`))
  (bind _returnvalue_4 (`|SpawnActorFromClass` (`self.BoardVisualiserClass`) (`KismetMathLibrary.MakeTransform` (0.0 0.0 0.0)) "Undefined" "MultiplyWithRoot" null null))
  (bind _output_get (set `self.BoardVisualiser` _returnvalue_4))
  (set `ABoardVisualiser.BoardManager` _returnvalue_2 _output_get)
  (set `ABoardVisualiser.TurnManager` _returnvalue_3 _output_get)
  (set `UBoardManager.TurnManager` _returnvalue_3 _returnvalue_2)
  (bind (_outrefineries _outmothershipp0 _outmothershipp1) (`ABoardVisualiser.SpawnBoard` _output_get))
  (set `self.Refineries` _outrefineries)
  (set `self.Mothership P0` _outmothershipp0)
  (set `self.Mothership P1` _outmothershipp1)
  (`/Engine/EditorBlueprintResources/StandardMacros.IsValid` _returnvalue
    (:`Is Valid`
      (`UBoardManager.InitializeBoard` _returnvalue (`self.Refineries`) (`self.Mothership P0`) (`self.Mothership P1`)))
    (:`Is Not Valid`
      (`KismetSystemLibrary.PrintString` "caca"))))

(fn `InitializeDecks`
  (bind _returnvalue (`self.GetDeckManager`))
  (`/Engine/EditorBlueprintResources/StandardMacros.IsValid` _returnvalue
    (:`Is Valid`
      (for _ (range (+ (`self.playerCount`) 1))
        (`DeckManager.InitializeDeck` _returnvalue 0 (`self.TempDeck`))))
    (:`Is Not Valid`
      (`KismetSystemLibrary.PrintString` "popo"))))

(fn `InitializePlayerPosition`
  (`SceneComponent.K2_SetWorldTransform` (`Character.CapsuleComponent` (cast `/Game/Dev/Blueprints/Player/BP_PlayerTest` (`GameplayStatics.GetPlayerCharacter` 0) :!pure true)) (`KismetMathLibrary.MakeTransform` (`ABoardVisualiser.GridToWorld` (`self.BoardVisualiser`) (make `IntPoint` 2 4))) false false))

(fn `InitializeTurnManager`
  (bind _returnvalue (`self.GetTurnManager`))
  (`/Engine/EditorBlueprintResources/StandardMacros.IsValid` _returnvalue
    (:`Is Valid`
      (`UTurnManager.InitializeGame` _returnvalue 0 (`self.playerCount`)))
    (:`Is Not Valid`
      (`KismetSystemLibrary.PrintString` "pipi"))))

(fn `UserConstructionScript`)