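; Player controller for a turn-based ship card board game, bridging game events to the in-game UI, sounds and debug messages.
; Local setup creates the HUD and places the pawn at per-player camera positions, then notifies the server.
; Left-click traces route ships, cells and motherships to click handlers, using a pending intent set by card selection or target prompts.
; Keys cycle the camera, end turns, open pause and request ship reveals.
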(event `self.ReceiveBeginPlay`
  ; BeginPlay
  (bind _returnvalue (`GameplayStatics.GetActorOfClass` "/Game/Managers/SoundManager/BP_SoundManager.BP_SoundManager_C"))
  (set `self.sound_manager` _returnvalue))

(event `HideShipStat`
  (`Widget.SetVisibility` (`/Game/Player/InGameWidget/UWB_InGameUI.UWB_Card` (`self.GameUi`)) "Hidden"))

(event `self.OnCardPlayedBP`
  ; When player play a card
  (`/Game/Cards/Widget/UWB_Card.RemoveCard` (`self.SelectedCardUI`))
  (`self.ClearSelection`)
  (`/Game/Managers/SoundManager/BP_SoundManager.PlaySFX` (`self.sound_manager`) null))

(event `self.OnCardDiscardedBP`
  (params (cardData :type "UCardData Object Reference"))
  (`/Game/Player/InGameWidget/UWB_InGameUI.DiscardCard` (`self.GameUi`) cardData))

(event `self.OnCardDrawnBP`
  (params (Card :type "UCardData Object Reference"))
  ; When card is drawn
  (`/Game/Player/InGameWidget/UWB_InGameUI.DrawCard` (`self.GameUi`) Card)
  (`/Game/Managers/SoundManager/BP_SoundManager.PlaySFX` (`self.sound_manager`) null))

(event `ShowShipStat`
  (params (Ship :type "AShip Object Reference"))
  (bind _uwb_card (`/Game/Player/InGameWidget/UWB_InGameUI.UWB_Card` (`self.GameUi`)))
  (`Widget.SetVisibility` _uwb_card "HitTestInvisible")
  (`/Game/Cards/Widget/UWB_Card.UpdateCard` _uwb_card Ship true))

(event `self.OnActionRejectedBP`
  (params (Reason :type String))
  (`KismetSystemLibrary.PrintString` Reason true true (struct :`R` 1.0 :`B` 0.047673 :`A` 1.0) 20.0))

(event `self.OnTurnStartedBP`
  (params (ActivePlayerID :type Integer) (bIsLocalPlayerTurn :type Boolean))
  ; When Turn Start
  (if bIsLocalPlayerTurn
    (`self.UpdateEssenceUi`)
    (`Widget.SetVisibility` (`/Game/Player/InGameWidget/UWB_InGameUI.Turn` (`self.GameUi`)) "Visible")
    (`/Game/Managers/SoundManager/BP_SoundManager.PlaySFX` (`self.sound_manager`) null)))

(event `self.OnVictoryBP`
  (params (WinnerID :type Integer))
  ; When Player win
  (`KismetSystemLibrary.PrintString` (`KismetStringLibrary.Concat_StrStr` "Le joueur  " (`KismetStringLibrary.Conv_IntToString` WinnerID) " à gagné !") true true (struct :`R` 1.0 :`G` 0.817859 :`A` 1.0) 50000.0)
  (if (== WinnerID (`self.PlayerID`))
    (`KismetSystemLibrary.PrintString` "Victoire !" true true (struct :`R` 0.155071 :`G` 1.0 :`A` 1.0) 50000.0)
    (else
      (`KismetSystemLibrary.PrintString` "Defaite !" true true (struct :`R` 1.0 :`G` 0.013328 :`A` 1.0) 50000.0)))
  (`/Game/Managers/SoundManager/BP_SoundManager.PlaySFX` (`self.sound_manager`) null))

(event `self.OnTurnEndedBP`
  ; When Turn End
  (`/Game/Managers/SoundManager/BP_SoundManager.PlaySFX` (`self.sound_manager`) null))

(event `self.OnShipDestroyedBP`
  (params (Ship :type "AShip Object Reference"))
  ; When ship is destroyed
  (`/Game/Managers/SoundManager/BP_SoundManager.PlaySFX` (`self.sound_manager`) null))

(event `self.OnEssenceChangedBP`
  (params (NewEssence :type Integer) (NewMaxEssence :type Integer))
  (`self.UpdateEssenceUi`))

(event `self.OnClearSelectionBP`
  (`/Game/Player/InGameWidget/UWB_InGameUI.ClearChoosableCards` (`self.GameUi`)))

(event `self.OnSabotageTargetPromptBP`
  (params (Candidates :type "Array of UCardData Object Reference (by ref)"))
  (`KismetSystemLibrary.PrintString` "Sabotage prompt" true true (struct :`R` 0.291771 :`B` 1.0 :`A` 1.0) 50.0)
  (set `self.PendingIntent` "ACTIVATE")
  (`/Game/Player/InGameWidget/UWB_InGameUI.SetChoosableCards` (`self.GameUi`) Candidates self))

(event `self.InitializeInputBP`
  (if (`self.IsLocalPlayerController` self)
    (`self.SetUpPlayerVar`)
    (bind _returnvalue (`|CreateWidget` "/Game/Player/InGameWidget/UWB_InGameUI.UWB_InGameUI_C" self))
    (set `/Game/Player/InGameWidget/UWB_InGameUI.Owner` self _returnvalue)
    (set `self.GameUi` _returnvalue)
    (`UserWidget.AddToViewport` _returnvalue 0)
    (`self.ServerSetupFinish`)))

(event `self.OnShipSelectedBP`
  (params (Ship :type "AShip Object Reference"))
  (`AShip.OnShipSelectedBP` Ship))

(event `self.OnEffectTargetPromptBP`
  (params (Kind :type "EEffectTargetKind Enum" :default "None"))
  (`KismetSystemLibrary.PrintString` "Effect prompt" true true (struct :`R` 0.291771 :`B` 1.0 :`A` 1.0) 50.0)
  (set `self.PendingIntent` "ACTIVATE"))

(event `EnhancedInput|/Game/Input/IA_LeftClick`
  (params (ActionValue :type Boolean) (ElapsedSeconds :type "Float (double-precision)") (TriggeredSeconds :type "Float (double-precision)") (InputAction :type "InputAction Object Reference" :default "/Game/Input/IA_LeftClick.IA_LeftClick"))
  (bind _hitresult (`self.GetHitResultUnderCursorByChannel` "TraceTypeQuery1"))
  (:`Started`
    (if (`|EnumInequality` (`self.PendingIntent`) "ACTIVATE")
      (bind _asbp_ship (cast `/Game/BoardActors/Ships/BP_Ship` (`.HitActor` (`GameplayStatics.BreakHitResult` _hitresult)))
        (:`then`
          (`self.ClickOnShip` _asbp_ship))
        (:`CastFailed`
          (bind _asbp_board_cell (cast `/Game/BoardActors/Cells/BP_BoardCell` (`.HitActor` (`GameplayStatics.BreakHitResult` _hitresult)))
            (:`then`
              (`self.ClickOnCell` _asbp_board_cell))
            (:`CastFailed`
              (bind _asbp_mother_ship (cast `/Game/BoardActors/MotherShip/BP_MotherShip` (`.HitActor` (`GameplayStatics.BreakHitResult` _hitresult)))
                (:`then`
                  (`self.ClickOnMotherShip` _asbp_mother_ship))
                (:`CastFailed`
                  (`self.ClearSelection`))))))))))

(event `SelectShip`
  (params (`Pending Ship Class` :type "AShip Class Reference") (`Card data` :type "UCardData Object Reference") (CardUI :type "/Game/Cards/Widget/UWB_Card Object Reference"))
  (set `self.PendingShipClass` `Pending Ship Class`)
  (set `self.PendingCardData` `Card data`)
  (set `self.PendingIntent` "PLAYCARD")
  (set `self.SelectedCardUI` CardUI))

(event `EnhancedInput|/Game/Input/IA_A`
  (params (ActionValue :type Boolean) (ElapsedSeconds :type "Float (double-precision)") (TriggeredSeconds :type "Float (double-precision)") (InputAction :type "InputAction Object Reference" :default "/Game/Input/IA_A.IA_A"))
  (:`Started`
    (`self.ChangeCameraAngle`)))

(event `EnhancedInput|/Game/Input/IA_E`
  (params (ActionValue :type Boolean) (ElapsedSeconds :type "Float (double-precision)") (TriggeredSeconds :type "Float (double-precision)") (InputAction :type "InputAction Object Reference" :default "/Game/Input/IA_E.IA_E"))
  (:`Started`
    (`self.ChangeCameraAngle`)))

(event `EnhancedInput|/Game/Input/IA_T`
  (params (ActionValue :type Boolean) (ElapsedSeconds :type "Float (double-precision)") (TriggeredSeconds :type "Float (double-precision)") (InputAction :type "InputAction Object Reference" :default "/Game/Input/IA_T.IA_T"))
  (:`Started`
    (`Widget.SetVisibility` (`/Game/Player/InGameWidget/UWB_InGameUI.Turn` (`self.GameUi`)) "Hidden")
    (`self.RequestEndTurn`)))

(event `EnhancedInput|/Game/Input/IA_Escape`
  (params (ActionValue :type Boolean) (ElapsedSeconds :type "Float (double-precision)") (TriggeredSeconds :type "Float (double-precision)") (InputAction :type "InputAction Object Reference" :default "/Game/Input/IA_Escape.IA_Escape"))
  (:`Started`
    (`/Engine/EditorBlueprintResources/StandardMacros.IsValid` (`self.PauseMenuRef`)
      (:`Is Valid`
        (if (`|EnumEquality` (`Widget.GetVisibility` (`self.PauseMenuRef`)) "Hidden")
          (`Widget.SetVisibility` (`self.PauseMenuRef`) "Visible")
          (`WidgetBlueprintLibrary.SetInputMode_UIOnlyEx` self null)))
      (:`Is Not Valid`
        (bind _returnvalue (`|CreateWidget` "/Game/Player/InGameWidget/UWP_PauseMenu.UWP_PauseMenu_C" self))
        (bind _output_get (set `self.PauseMenuRef` _returnvalue))
        (`UserWidget.AddToViewport` _output_get 0)
        (`WidgetBlueprintLibrary.SetInputMode_UIOnlyEx` null null)))))

(event `EnhancedInput|/Game/Input/IA_R`
  (params (ActionValue :type Boolean) (ElapsedSeconds :type "Float (double-precision)") (TriggeredSeconds :type "Float (double-precision)") (InputAction :type "InputAction Object Reference" :default "/Game/Input/IA_R.IA_R"))
  (bind _selectedship (`self.SelectedShip`))
  (:`Started`
    (`/Engine/EditorBlueprintResources/StandardMacros.IsValid` _selectedship
      (:`Is Valid`
        (`self.Server_RevealShip` _selectedship)))))

(fn `ChangeCameraAngle`
  (bind _output_playertransforms (break `/Game/Core/TransformVector` (`|GetArrayItem` (`self.PlayerBoardPosition`) (`self.PlayerID`))))
  (bind (_output_location _output_rotation) (`KismetMathLibrary.BreakTransform` (`|GetArrayItem` _output_playertransforms (`self.CameraAngleIndex`))))
  (bind _result (`/Engine/EditorBlueprintResources/StandardMacros.IncrementInt` (`self.CameraAngleIndex`))
    (:`  `
      (if (>= _result (`KismetArrayLibrary.Array_Length` _output_playertransforms))
        (set `self.CameraAngleIndex` 0))
      (`self.K2_SetActorLocationAndRotation` (`self.PlayerRef`) _output_location _output_rotation false false))))

(fn `SetUpPlayerVar`
  (bind _asc_player (cast `/Game/Player/C_Player` (`self.K2_GetPawn`))
    (:`then`
      (set `self.PlayerRef` _asc_player)
      (`self.ChangeCameraAngle`))
    (:`CastFailed`
      (`KismetSystemLibrary.PrintString` "fail")
      (`KismetSystemLibrary.K2_SetTimer` null "SetUpPlayerVar" 1.0))))

(fn `UpdateEssenceUi`
  (bind _gameui (`self.GameUi`))
  (bind _asboard_player_state (cast `BoardPlayerState` (`self.PlayerState`)))
  (`/Engine/EditorBlueprintResources/StandardMacros.IsValid` _gameui
    (:`Is Valid`
      (`/Game/Player/InGameWidget/UWB_InGameUI.UpdateEssence` _gameui (`BoardPlayerState.CurrentEssence` _asboard_player_state) (`BoardPlayerState.MaxEssence` _asboard_player_state) (`BoardPlayerState.BonusEssence` _asboard_player_state)))))

(fn `UserConstructionScript`)