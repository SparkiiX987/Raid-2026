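; GM_BoardGameMode is the game mode that sets up the board and mouse input when play begins.
; It spawns a BP_BoardVisualiser, whose SpawnBoard creates the board and returns refineries and motherships for P0 and P1.
; It passes those results to UBoardManager to initialize the board, then enables the cursor and click events for player controller 0.
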(event `self.ReceiveBeginPlay`
  (bind _returnvalue (`GameplayStatics.GetPlayerController` 0))
  (bind _returnvalue_2 (`|SpawnActorFromClass` "/Game/BP_BoardVisualiser.BP_BoardVisualiser_C" (`KismetMathLibrary.MakeTransform` (0.0 0.0 0.0)) "Undefined" "MultiplyWithRoot" null null))
  (bind (_outrefineries _outmothershipp0 _outmothershipp1) (`ABoardVisualiser.SpawnBoard` _returnvalue_2))
  (set `self.Refineries` _outrefineries)
  (set `self.Mothership P0` _outmothershipp0)
  (set `self.Mothership P1` _outmothershipp1)
  (`UBoardManager.InitializeBoard` (subsystem `UBoardManager`) (`self.Refineries`) (`self.Mothership P0`) (`self.Mothership P1`))
  (set `PlayerController.bShowMouseCursor` true _returnvalue)
  (set `PlayerController.bEnableClickEvents` true _returnvalue))

(fn `UserConstructionScript`)