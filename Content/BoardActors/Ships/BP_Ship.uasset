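; Board-game ship actor that presents a card-driven ship, playing sounds through BP_SoundManager on spawn, move, action and damage.
; Spawn takes the mesh from card data with a background material, reveal recolors by owner, and RepNotifies apply both, rotating player 1's ship.
; Selection swaps in a highlight material.
; A timed cursor hover shows stats through the board player controller, limited to the owner while face down.
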(event `self.ReceiveBeginPlay`
  ; Begin play
  (bind _returnvalue (`GameplayStatics.GetActorOfClass` "/Game/Managers/SoundManager/BP_SoundManager.BP_SoundManager_C"))
  (set `self.Sound_Manager` _returnvalue))

(event `self.OnActorDamagedBP`
  ; ShipSfx
  (`/Game/Managers/SoundManager/BP_SoundManager.PlaySFX` (`self.Sound_Manager`) null))

(event `self.OnActBP`
  ; ShipSfx
  (`/Game/Managers/SoundManager/BP_SoundManager.PlaySFX` (`self.Sound_Manager`) null))

(event `self.OnShipSpawnBP`
  ; when ship is spawned
  (set `self.ShipMesh` (`UCardData.shipMesh` (`self.CardData`)))
  (set `self.ShipMaterial` "/Engine/EngineMeshes/BackgroundMaterial.BackgroundMaterial")
  (`/Game/Managers/SoundManager/BP_SoundManager.PlaySFX` (`self.Sound_Manager`) null))

(event `self.OnMoveBP`
  ; ShipSfx
  (`/Game/Managers/SoundManager/BP_SoundManager.PlaySFX` (`self.Sound_Manager`) null))

(event `self.OnShipSelectedBP`
  (`PrimitiveComponent.SetMaterial` (`self.Cube`) 0 (`self.ShipHighlightMaterial`)))

(event `self.OnShipUnselectedBP`
  (`PrimitiveComponent.SetMaterial` (`self.Cube`) 0 (`self.ShipMaterial`)))

(event `self.Cube.OnBeginCursorOver`
  (params (TouchedComponent :type "PrimitiveComponent Object Reference"))
  (bind _returnvalue (`KismetSystemLibrary.K2_SetTimerDelegate` (delegate `ShowStats`) 1.0))
  (set `self.TimerForHover` _returnvalue))

(event `ShowStats`
  (bind _aspc_board_player_controller (cast `/Game/Player/PlayerController/PC_BoardPlayerController` (`GameplayStatics.GetPlayerController` 0)))
  (if (`self.IsFaceDown`)
    (if (== (`self.GetOwnerID`) (`BoardPlayerController.PlayerID` _aspc_board_player_controller))
      (`/Game/Player/PlayerController/PC_BoardPlayerController.ShowShipStat` _aspc_board_player_controller self :!label _label))
    (else
      (goto _label))))

(event `self.Cube.OnEndCursorOver`
  (params (TouchedComponent :type "PrimitiveComponent Object Reference"))
  (`KismetSystemLibrary.K2_ClearAndInvalidateTimerHandle` (`self.TimerForHover`))
  (bind _aspc_board_player_controller (cast `/Game/Player/PlayerController/PC_BoardPlayerController` (`GameplayStatics.GetPlayerController` 0)))
  (`/Game/Player/PlayerController/PC_BoardPlayerController.HideShipStat` _aspc_board_player_controller))

(event `self.PlayRevealAnimation`
  (if (== (`self.GetOwnerID`) 0)
    (set `self.ShipMaterial` "/Game/BoardActors/Ships/Materials/M_Blue.M_Blue")
    (else
      (set `self.ShipMaterial` "/Game/BoardActors/Ships/Materials/M_Red.M_Red"))))

(fn `OnRep_ShipMaterial`
  (`PrimitiveComponent.SetMaterial` (`self.Cube`) 0 (`self.ShipMaterial`)))

(fn `OnRep_ShipMesh`
  (`StaticMeshComponent.SetStaticMesh` (`self.Cube`) (`self.ShipMesh`))
  (if (== (`self.GetOwnerID`) 1)
    (`self.K2_SetActorRotation` (struct :`Yaw` 180.0))))

(fn `UserConstructionScript`)