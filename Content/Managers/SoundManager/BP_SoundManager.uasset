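; BP_SoundManager is a sound manager that plays recurring random ambient sounds and on-demand sound effects, all as non-spatialized 2D audio.
; BeginPlay starts AmbientSFX, which plays a random Sound array entry, waits a minute, then calls itself to loop.
; The random index range includes the array length, so it can land one past the last entry.
; A separate PlaySFX event plays whatever sound is passed to it.
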(event `Ambient SFX`
  (`GameplayStatics.PlaySound2D` (`|GetArrayItem` (`self.Sound`) (`KismetMathLibrary.RandomIntegerInRange` 0 (`KismetArrayLibrary.Array_Length` (`self.Sound`)))) 1.0 1.0 0.0 null null)
  (`KismetSystemLibrary.Delay` 60.0)
  (`self.Ambient SFX`))

(event `self.ReceiveBeginPlay`
  (`self.Ambient SFX`))

(event `PlaySFX`
  (params (NewParam :type "SoundBase Object Reference"))
  (`GameplayStatics.PlaySound2D` NewParam 1.0 1.0 0.0 null null))

(fn `UserConstructionScript`)